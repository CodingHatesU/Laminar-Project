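; PlaneBP is an actor set up to fly along the spline of a SplinePathBP found in the level.
; On BeginPlay it stores that path and plays MoveObjectTimeline at a rate of one over TTCInSeconds.
; A SetActorTransform maps the timeline track to distance along the spline, taking world-space location and local-space rotation.
; That transform node is unwired and never runs, so the timeline does not move the plane.
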(event Custom|Move%20Object
  (Components|Timeline|SetPlayRate (Variables|Default|GetMove%20Object%20Timeline) (/ 1.0 (Variables|Default|GetTTC%20%28In%20Seconds%29)))
  (bind _newtrack_0 (Timeline|Move%20Object%20Timeline Play)))

(event EventBeginPlay
  (bind _returnvalue (Actor|GetActorOfClass "/Game/SplinePathBP.SplinePathBP_C"))
  (Variables|Default|SetSpline%20REF _returnvalue)
  (CallFunction|MoveObject))

(fn ConstructionScript)